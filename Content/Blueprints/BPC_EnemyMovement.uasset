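; Actor component that patrols its owning Pawn back and forth along X between its start position and EndLocationX.
; A looping timer calls MovePawn, which uses the Reverse flag to step the transform forward or back, flipping on exact position matches.
; RotateEnemyToFacePlayer, not called here, toggles Reverse when pawn yaw differs from the passed object's control yaw, without directly rotating anything.
; TravelDistance is calculated at BeginPlay but unused.
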(event `self.ReceiveBeginPlay`
  (bind _aspawn (cast `Pawn` (`self.GetOwner`)))
  (bind _output_get (set `self.PawnRef` _aspawn))
  (bind _returnvalue_x (`KismetMathLibrary.BreakVector` (`Actor.K2_GetActorLocation` _output_get)))
  (set `self.StartLocation` _returnvalue_x)
  (if (< (`self.StartLocation`) 0.0)
    (set `self.TravelDistance` (+ (`self.StartLocation`) (`self.EndLocationX`)))
    (else
      (set `self.TravelDistance` (- (`self.StartLocation`) (`self.EndLocationX`)))))
  (bind _returnvalue (`KismetSystemLibrary.K2_SetTimer` null "MovePawn" 0.05 true))
  (set `self.TimerRef` _returnvalue))

(fn `MovePawn`
  (bind _pawnref (`self.PawnRef`))
  (bind (_returnvalue_x _returnvalue_y _returnvalue_z) (`KismetMathLibrary.BreakVector` (`Actor.K2_GetActorLocation` _pawnref)))
  (set `self.CurrentLocationX` _returnvalue_x)
  (if (`self.Reverse?`)
    (`self.TravelBack` _pawnref _returnvalue_y _returnvalue_z)
    (else
      (`self.TravelForward` _pawnref _returnvalue_y _returnvalue_z))))

(fn `RotateEnemyToFacePlayer`
  (params (self2 :type "Pawn Object Reference"))
  (if (== (.yaw (`Actor.K2_GetActorRotation` (`self.PawnRef`))) (.yaw (`Pawn.GetControlRotation` self2)))
    (`KismetSystemLibrary.PrintString` "Facing Player")
    (else
      (`KismetSystemLibrary.PrintString` "NOT facing player")
      (if (`self.Reverse?`)
        (set `self.Reverse?` false)
        (else
          (set `self.Reverse?` true)))))
  (return))

(fn `TravelBack`
  (params (self2 :type "Actor Object Reference") (NewTransform_Location_Y :type "Float (double-precision)") (NewTransform_Location_Z :type "Float (double-precision)"))
  (`Actor.K2_SetActorTransform` self2 (`KismetMathLibrary.MakeTransform` (`KismetMathLibrary.MakeVector` (+ (`self.CurrentLocationX`) (`self.DistancePerTick`)) NewTransform_Location_Y NewTransform_Location_Z) (struct :`Yaw` 180.0)) false false)
  (if (== (`self.CurrentLocationX`) (`self.StartLocation`))
    (set `self.Reverse?` false)
    (else
      (set `self.Reverse?` true))))

(fn `TravelForward`
  (params (self2 :type "Actor Object Reference") (NewTransform_Location_Y :type "Float (double-precision)") (NewTransform_Location_Z :type "Float (double-precision)"))
  (`Actor.K2_SetActorTransform` self2 (`KismetMathLibrary.MakeTransform` (`KismetMathLibrary.MakeVector` (- (`self.CurrentLocationX`) (`self.DistancePerTick`)) NewTransform_Location_Y NewTransform_Location_Z)) false false)
  (if (== (`self.CurrentLocationX`) (`self.EndLocationX`))
    (set `self.Reverse?` true)
    (else
      (set `self.Reverse?` false))))