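; Enemy attack component that applies an enemy's per-hit damage to the player's health.
; On BeginPlay it caches its owning BP_MyEnemy and the player's BP_MyCharacter.
; UpdatePlayerHealth returns true when the hit would bring health to zero or below, leaving Health unchanged; otherwise it subtracts the damage and returns false.
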(event `self.ReceiveBeginPlay`
  (bind _asbp_my_enemy (cast `/Game/Blueprints/BP_MyEnemy` (`self.GetOwner`)))
  (set `self.EnemyRef` _asbp_my_enemy)
  (bind _asbp_my_character (cast `/Game/Blueprints/BP_MyCharacter` (`GameplayStatics.GetPlayerCharacter` 0)))
  (set `self.PlayerCharRef` _asbp_my_character))

(fn `UpdatePlayerHealth`
  (returns (`Dead?` :type Boolean))
  (bind _playercharref (`self.PlayerCharRef`))
  (bind _returnvalue (- (`/Game/Blueprints/BP_MyCharacter.Health` _playercharref) (`/Game/Blueprints/BP_MyEnemy.DamagePerHit` (`self.EnemyRef`))))
  (if (<= _returnvalue 0.0)
    (return true)
    (else
      (set `/Game/Blueprints/BP_MyCharacter.Health` _returnvalue _playercharref)
      (return false))))