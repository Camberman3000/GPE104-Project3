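; BP_Enemy is a bee enemy that warns when the player comes near and kills and respawns them on a bite.
; DangerSphere overlap speeds up the bee animation and plays an angry buzz until overlap ends.
; BiteSphere overlap halts the player and pauses the BPCEnemyMovement timer until overlap ends.
; After a short delay it destroys the character, then spawns and possesses a new one at the first PlayerStart found.
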(event `self.DangerSphere.OnComponentBeginOverlap`
  (params (OverlappedComponent :type "PrimitiveComponent Object Reference") (OtherActor :type "Actor Object Reference") (OtherComp :type "PrimitiveComponent Object Reference") (OtherBodyIndex :type Integer) (bFromSweep :type Boolean) (SweepResult :type "HitResult Structure (by ref)"))
  (cast `/Game/Blueprints/BP_MyCharacter` (`.HitActor` (`GameplayStatics.BreakHitResult` SweepResult)))
  (`KismetSystemLibrary.PrintString` "DANGER!!")
  (`PaperFlipbookComponent.SetPlayRate` (`self.bee_animation`) 12.0)
  (bind _returnvalue (`GameplayStatics.SpawnSound2D` "/Game/Sounds/angrybee.angrybee" 1.0 1.0 0.0 null))
  (set `self.AngryBeeSoundRef` _returnvalue))

(event `self.DangerSphere.OnComponentEndOverlap`
  (params (OverlappedComponent :type "PrimitiveComponent Object Reference") (OtherActor :type "Actor Object Reference") (OtherComp :type "PrimitiveComponent Object Reference") (OtherBodyIndex :type Integer))
  (bind _angrybeesoundref (`self.AngryBeeSoundRef`))
  (`PaperFlipbookComponent.SetPlayRate` (`self.bee_animation`) 1.0)
  (`/Engine/EditorBlueprintResources/StandardMacros.IsValid` _angrybeesoundref
    (:`Is Valid`
      (`AudioComponent.Stop` _angrybeesoundref))))

(event `self.BiteSphere.OnComponentBeginOverlap`
  (params (OverlappedComponent :type "PrimitiveComponent Object Reference") (OtherActor :type "Actor Object Reference") (OtherComp :type "PrimitiveComponent Object Reference") (OtherBodyIndex :type Integer) (bFromSweep :type Boolean) (SweepResult :type "HitResult Structure (by ref)"))
  (bind _asbp_my_character (cast `/Game/Blueprints/BP_MyCharacter` OtherActor))
  (`KismetSystemLibrary.PrintString` "I'M HIT. OW!")
  (bind _charactermovement (`Character.CharacterMovement` _asbp_my_character))
  (`MovementComponent.StopMovementImmediately` _charactermovement)
  (`PaperFlipbookComponent.SetPlayRate` (`self.bee_animation`) 12.0)
  (`KismetSystemLibrary.K2_PauseTimerHandle` (`/Game/Blueprints/BPC_EnemyMovement.TimerRef` (`self.BPC_EnemyMovement`)))
  (bind _returnvalue (`GameplayStatics.SpawnSound2D` "/Game/Sounds/angrybee.angrybee" 1.0 1.0 0.0 null))
  (set `self.AngryBeeSoundRef` _returnvalue)
  (`KismetSystemLibrary.Delay` 1.0)
  (`CharacterMovementComponent.SetMovementMode` _charactermovement "MOVE_Walking" 0)
  (`self.K2_DestroyActor` _asbp_my_character)
  (`AudioComponent.Stop` (`self.AngryBeeSoundRef`))
  (`PaperFlipbookComponent.SetPlayRate` (`self.bee_animation`) 1.0)
  (bind _outactors (`GameplayStatics.GetAllActorsOfClass` "/Script/Engine.PlayerStart"))
  (bind _returnvalue_2 (`|SpawnActorFromClass` "/Game/Blueprints/BP_MyCharacter.BP_MyCharacter_C" (`KismetMathLibrary.MakeTransform` (`self.K2_GetActorLocation` (`|GetArrayItem` _outactors))) "Undefined" "OverrideRootScale" null null))
  (`Controller.Possess` (`GameplayStatics.GetPlayerController` 0) _returnvalue_2))

(event `self.BiteSphere.OnComponentEndOverlap`
  (params (OverlappedComponent :type "PrimitiveComponent Object Reference") (OtherActor :type "Actor Object Reference") (OtherComp :type "PrimitiveComponent Object Reference") (OtherBodyIndex :type Integer))
  (`KismetSystemLibrary.K2_UnPauseTimerHandle` (`/Game/Blueprints/BPC_EnemyMovement.TimerRef` (`self.BPC_EnemyMovement`)))
  (`PaperFlipbookComponent.SetPlayRate` (`self.bee_animation`) 1.0))

(fn `UserConstructionScript`)