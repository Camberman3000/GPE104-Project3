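; BP_Slime is a slime enemy that warns of and attacks the player through two overlap spheres, delegating to movement, animation, sound and attack components.
; Entering DangerSphere turns it toward the player, speeds its animation and plays a warning sound.
; Entering AttackSphere attacks if CanAttack is set, pausing the movement timer and updating health, then destroying and respawning the player on death.
; CanAttack re-arms upon leaving DangerSphere or player death.
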(event `self.ReceiveBeginPlay`
  (bind _asbp_my_character (cast `/Game/Blueprints/Player/BP_MyCharacter` (`GameplayStatics.GetPlayerCharacter` 0)))
  (set `self.PlayerCharRef` _asbp_my_character)
  (bind _asbp_player_controller (cast `/Game/Blueprints/Player/BP_PlayerController` (`GameplayStatics.GetPlayerController` 0)))
  (set `self.PlayerControllerRef` _asbp_player_controller))

(event `self.DangerSphere.OnComponentBeginOverlap`
  (params (OverlappedComponent :type "PrimitiveComponent Object Reference") (OtherActor :type "Actor Object Reference") (OtherComp :type "PrimitiveComponent Object Reference") (OtherBodyIndex :type Integer) (bFromSweep :type Boolean) (SweepResult :type "HitResult Structure (by ref)"))
  ;[1 0.8922 0] Danger Sphere overlap
  (bind _asbp_my_character (cast `/Game/Blueprints/Player/BP_MyCharacter` OtherActor))
  (bind _output_get (set `self.PlayerCharRef` _asbp_my_character))
  (`/Game/Blueprints/Enemy/BPC_EnemyMovement.RotateEnemyToFacePlayer` (`self.BPC_EnemyMovement`) _output_get)
  (`/Game/Blueprints/Enemy/BPC_EnemyAnimation.SetEnemyAnimSpeed` (`self.BPC_EnemyAnimation`) (`self.AnimFastSpeed`))
  (`/Game/Blueprints/Enemy/BPC_EnemySounds.PlaySound` (`self.BPC_EnemySounds`) (`self.DangerSoundToPlay`)))

(event `self.DangerSphere.OnComponentEndOverlap`
  (params (OverlappedComponent :type "PrimitiveComponent Object Reference") (OtherActor :type "Actor Object Reference") (OtherComp :type "PrimitiveComponent Object Reference") (OtherBodyIndex :type Integer))
  ;[1 0.8922 0] Danger Sphere overlap
  (cast `/Game/Blueprints/Player/BP_MyCharacter` OtherActor)
  (`/Game/Blueprints/Enemy/BPC_EnemyAnimation.SetEnemyAnimSpeed` (`self.BPC_EnemyAnimation`) (`self.AnimSlowSpeed`))
  (set `self.CanAttack?` true)
  (`/Game/Blueprints/Enemy/BPC_EnemySounds.StopSound` (`self.BPC_EnemySounds`) (`/Game/Blueprints/Enemy/BPC_EnemySounds.DangerSoundRef` (`self.BPC_EnemySounds`))))

(event `self.AttackSphere.OnComponentBeginOverlap`
  (params (OverlappedComponent :type "PrimitiveComponent Object Reference") (OtherActor :type "Actor Object Reference") (OtherComp :type "PrimitiveComponent Object Reference") (OtherBodyIndex :type Integer) (bFromSweep :type Boolean) (SweepResult :type "HitResult Structure (by ref)"))
  (bind _bpc_enemysounds (`self.BPC_EnemySounds`))
  (bind _bpc_enemysounds_2 (`self.BPC_EnemySounds`))
  ;[1 0 0] Attack Sphere Overlap
  (bind _asbp_my_character (cast `/Game/Blueprints/Player/BP_MyCharacter` OtherActor))
  (set `self.PlayerCharRef` _asbp_my_character)
  (`/Game/Blueprints/Enemy/BPC_EnemySounds.StopSound` _bpc_enemysounds (`/Game/Blueprints/Enemy/BPC_EnemySounds.DangerSoundRef` _bpc_enemysounds))
  (if (`self.CanAttack?`)
    (set `self.CanAttack?` false)
    (`KismetSystemLibrary.PrintString` "I'M HIT. OW!")
    (`KismetSystemLibrary.K2_PauseTimerHandle` (`/Game/Blueprints/Enemy/BPC_EnemyMovement.TimerRef` (`self.BPC_EnemyMovement`)))
    (`/Game/Blueprints/Enemy/BPC_EnemySounds.StopSound` _bpc_enemysounds_2 (`/Game/Blueprints/Enemy/BPC_EnemySounds.DangerSoundRef` _bpc_enemysounds_2)) ; Stop Danger sound
    (`/Game/Blueprints/Enemy/BPC_EnemySounds.PlaySound` (`self.BPC_EnemySounds`) (`self.AttackSoundToPlay`))
    (bind _dead_ (`/Game/Blueprints/Enemy/BPC_EnemyAttack.UpdatePlayerHealth` (`self.BPC_EnemyAttack`)))
    (if _dead_
      (`self.K2_DestroyActor` (`self.PlayerCharRef`))
      (`/Game/Blueprints/Player/BP_PlayerController.Respawn` (`self.PlayerControllerRef`))
      (set `self.CanAttack?` true)
      (else
        (`/Game/Blueprints/Enemy/BPC_EnemyAnimation.SetEnemyAnimSpeed` (`self.BPC_EnemyAnimation`) (`self.AnimSlowSpeed`))))))

(event `self.AttackSphere.OnComponentEndOverlap`
  (params (OverlappedComponent :type "PrimitiveComponent Object Reference") (OtherActor :type "Actor Object Reference") (OtherComp :type "PrimitiveComponent Object Reference") (OtherBodyIndex :type Integer))
  ;[1 0 0] Attack Sphere Overlap
  (cast `/Game/Blueprints/Player/BP_MyCharacter` OtherActor)
  (`KismetSystemLibrary.K2_UnPauseTimerHandle` (`/Game/Blueprints/Enemy/BPC_EnemyMovement.TimerRef` (`self.BPC_EnemyMovement`)))
  (`/Game/Blueprints/Enemy/BPC_EnemyAnimation.SetEnemyAnimSpeed` (`self.BPC_EnemyAnimation`) (`self.AnimSlowSpeed`)))

(fn `UserConstructionScript`)